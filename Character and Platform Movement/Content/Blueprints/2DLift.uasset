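; A 2D sprite lift that travels between its origin and an end location, with timeline speed set from a travel time.
; The timeline lerps the sprite's position and, on finishing, waits a stop delay before running the opposite way.
; A safety collider reacts to the player character during movement, but its hard-wired true branch always calls Play, leaving Reverse unreachable.
; The construction script applies the color and can preview the end position.
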(event `self.ReceiveActorBeginOverlap`
  (params (OtherActor :type "Actor Object Reference")))

(event `self.ReceiveTick`
  (params (DeltaSeconds :type "Float (single-precision)")))

(event `self.ReceiveBeginPlay`
  ;[1 1 1] Time handling
  (`TimelineComponent.SetPlayRate` (`self.LiftTimeline`) (/ 1.0 (`self.TravelTimeInSeconds`)))
  (set `self.TestEndLocation` true))

(event `self.SafetyCollider.OnComponentBeginOverlap`
  (params (OtherActor :type "Actor Object Reference") (OtherComp :type "PrimitiveComponent Object Reference") (OtherBodyIndex :type Integer) (bFromSweep :type Boolean) (SweepResult :type "EngineTypes.HitResult Structure (by ref)"))
  ;[1 1 1] Collision handling
  (cast `/Game/Blueprints/MyCharacter` OtherActor)
  (if (`ActorComponent.IsActive` (`self.LiftTimeline`))
    (if true
      ;[1 1 1] Direction changing
      (bind (_direction _lerp_alpha) (`Timeline|LiftTimeline` :!label _label)
        (:`Update`
          (`SceneComponent.K2_SetRelativeLocation` (`self.LiftSprite`) (`KismetMathLibrary.VLerp` (0.0 0.0 0.0) (`self.EndLocation`) _lerp_alpha) false))
        (:`Finished`
          (`KismetSystemLibrary.Delay` (`self.StopDelay`))
          (switch `TimelineComponent.ETimelineDirection` _direction
            (:`Forward`
              (`self.LiftBackward`))
            (:`Backward`
              (`self.LiftForward`)))))
      (else
        (goto _label :!via `Reverse`)))))

(event `LiftForward`
  ;[1 1 1] Direction changing
  (goto _label :!via `PlayFromStart`))

(event `LiftBackward`
  ;[1 1 1] Direction changing
  (goto _label :!via `ReverseFromEnd`))

(fn `UserConstructionScript`
  (bind _liftsprite (`self.LiftSprite`))
  (`SceneComponent.K2_SetRelativeLocation` _liftsprite (`KismetMathLibrary.SelectVector` (`self.EndLocation`) (0.0 0.0 0.0) (`self.TestEndLocation`)) false)
  (`PaperSpriteComponent.SetSpriteColor` _liftsprite (`self.LiftColor`)))