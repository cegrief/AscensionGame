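; Paper2D side-scrolling player character that jumps, moves along world X and swaps sprite animations.
; The MoveRight axis adds movement, flips controller yaw to face the input direction and calls UpdateAnimation, so Tick stays unused.
; UpdateAnimation passes velocity and falling checks to a small state-machine function that picks the idle, running or jumping flipbook, with falling taking priority.
; BeginPlay explicitly disables replication.
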(event Custom|Update%20Animation
  ;[1 1 1] Animation Handling
  (Variables|Default|SetIs%20moving (> (Math|Vector|VectorLength (Transformation|GetVelocity)) 0.0))
  (Variables|Default|SetIs%20Falling (AI|Components|NavMovement|IsFalling (Variables|Character|GetCharacterMovement)))
  (bind _output_flipbook (CallFunction|AnimationStateMachine (Variables|Default|GetIs%20Falling) (Variables|Default|GetIs%20moving)))
  (Sprite|SetFlipbook (Variables|Default|GetSprite) _output_flipbook))

(event EventActorBeginOverlap
  (params (OtherActor :type Actor%20Object%20Reference)))

(event EventBeginPlay
  ;[1 1 1] Multiplayer possibility
  (Class|ActorComponent|SetIsReplicated false))

(event EventTick
  (params (DeltaSeconds :type Float%20%28single-precision%29)))

(event Input|ActionEvents|InputActionJump
  ;[1 1 1] Jumping
  (:Pressed
    (Character|Jump)))

(event Input|AxisEvents|InputAxisMoveRight
  (params (AxisValue :type Float%20%28single-precision%29))
  ;[1 1 1] Movement
  (Pawn|Input|AddMovementInput "1.000000, 0, 0" AxisValue false)
  (CallFunction|UpdateAnimation)
  (Math|Float|CompareFloat AxisValue 0.0
    (:>
      (Pawn|SetControlRotation (Pawn|GetController) (Class|KismetMathLibrary|MakeRot 0.0 0.0 0.0)))
    (:<
      (Pawn|SetControlRotation (Pawn|GetController) (Class|KismetMathLibrary|MakeRot 0.0 1.8e+02 0.0)))))

(fn ConstructionScript)

(fn AnimationStateMachine
  (params (IsFalling :type Boolean :default false) (IsMoving :type Boolean :default false))
  ;[1 1 1] Collect data
  (LocalVariables|SetIsFallingLocal IsFalling)
  (LocalVariables|SetIsMovingLocal IsMoving)
  ;[1 1 1] Test data
  (|TestForJumping
    (:then
      ;[1 1 1] Set Animation State
      (LocalVariables|SetAnimationState "NewEnumerator2"))
    (:else
      (|TestForRunningorIdle
        (:then
          (LocalVariables|SetAnimationState "NewEnumerator1"))
        (:else
          (LocalVariables|SetAnimationState "NewEnumerator0")))))
  (return (Utilities|Select :Index (LocalVariables|GetAnimationState) :NewEnumerator0 (Variables|Animations|GetIdleFlipbook) :NewEnumerator1 (Variables|Animations|GetRunFlipbook) :NewEnumerator2 (Variables|Animations|GetJumpFlipbook))))