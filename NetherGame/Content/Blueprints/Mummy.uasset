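; Mummy enemy Blueprint that applies point damage to MyCharacter on hit, with no damage amount set, and tracks its own health.
; Construction initializes HP and MaxHP, and AnyDamage subtracts incoming damage from HP.
; UpdateHPBar writes the health ratio to an enemyHealth widget, but nothing here calls it.
; Movement toward the player is unfinished: Tick only checks range, and direction and impulse-like vector math is left unconnected.
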(event `self.ReceiveHit`
  (params (MyComp :type "PrimitiveComponent Object Reference") (Other :type "Actor Object Reference") (OtherComp :type "PrimitiveComponent Object Reference") (bSelfMoved :type Boolean) (HitLocation :type "Object.Vector Structure") (HitNormal :type "Object.Vector Structure") (NormalImpulse :type "Object.Vector Structure") (Hit :type "EngineTypes.HitResult Structure (by ref)"))
  ;[1 1 1] Apply damage to things it touches
  (cast `/Game/Blueprints/MyCharacter` Other)
  (`GameplayStatics.ApplyPointDamage` Other 0.0 HitNormal Hit null self))

(event `self.ReceiveAnyDamage`
  (params (Damage :type "Float (single-precision)") (DamageType :type "DamageType Object Reference") (InstigatedBy :type "Controller Object Reference") (DamageCauser :type "Actor Object Reference"))
  (set `self.HP` (- (`self.HP`) Damage)))

(event `self.ReceiveTick`
  (params (DeltaSeconds :type "Float (single-precision)"))
  ;[1 1 1] Move Towards Player
  (if (<= (`self.GetDistanceTo` (`GameplayStatics.GetPlayerCharacter` 0)) 750.0)
    _))

(event `self.ReceiveBeginPlay`)

(event `self.ReceiveActorBeginOverlap`
  (params (OtherActor :type "Actor Object Reference")))

(fn `UpdateHPBar`
  (bind _asenemy_health (cast `/Game/Blueprints/enemyHealth` (`WidgetComponent.GetUserWidgetObject`)))
  (`ProgressBar.SetPercent` (`/Game/Blueprints/enemyHealth.hpBar` _asenemy_health) (/ (`self.HP`) (`self.MaxHP`))))

(fn `UserConstructionScript`
  (set `self.HP` 100.0)
  (set `self.MaxHP` 100.0))