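; Paper2D player character for a side-scrolling game, with running, double jump, sword attacks, sounds and death with level restart.
; Attacks apply damage to characters overlapping two sword hitboxes after a flipbook-timed delay.
; Point damage triggers knockback, red flash and explosion, and updates health in the Ascension game instance, which seeds it at construction.
; A prioritized state function (death, attack, jump, run, idle) selects the sprite flipbook.
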(event OnComponentHit(Cube)
  (params (OtherActor :type Actor%20Object%20Reference) (OtherComp :type Primitive%20Component%20Object%20Reference) (NormalImpulse :type Vector :default "0, 0, 0") (Hit :type Hit%20Result%20Structure%20%28by%20ref%29))
  (Development|PrintString "Hello"))

(event Custom|Update%20Animation
  ;[1 1 1] Animation Handling
  (Variables|Default|SetIs%20moving (> (Math|Vector|VectorLength (Transformation|GetVelocity)) 0.0))
  (Variables|Default|SetIs%20Falling (AI|Components|NavMovement|IsFalling (Variables|Character|GetCharacterMovement)))
  (bind _output_flipbook (CallFunction|AnimationStateMachine (Variables|Default|GetIs%20Falling) (Variables|Default|GetIs%20moving) (Variables|Default|GetIsDead) (Variables|Default|GetIs%20Attacking)))
  (Sprite|SetFlipbook (Variables|Default|GetSprite) _output_flipbook))

(event Custom|SwordHit
  (params (Damaged%20Actor :type Actor%20Object%20Reference))
  ;[1 1 1] Hit something with sword
  (Game|Damage|ApplyDamage Damaged%20Actor 5e+01 0 self))

(event EventActorBeginOverlap
  (params (OtherActor :type Actor%20Object%20Reference)))

(event EventBeginPlay
  ;[1 1 1] Add Health Display
  (bind _returnvalue (UserInterface|CreateWidget "/Game/Blueprints/CharacterHealth.CharacterHealth_C" (Game|GetPlayerController 0)))
  (UserInterface|Viewport|AddtoViewport _returnvalue 0))

(event EventPointDamage
  (params (Damage :type Float%20%28single-precision%29) (DamageType :type Damage%20Type%20Object%20Reference) (HitLocation :type Vector :default "0, 0, 0") (HitNormal :type Vector :default "0, 0, 0") (HitComponent :type Primitive%20Component%20Object%20Reference) (BoneName :type Name :default "None") (ShotFromDirection :type Vector :default "0, 0, 0") (InstigatedBy :type Controller%20Object%20Reference) (DamageCauser :type Actor%20Object%20Reference))
  ;[1 1 1] Take Damage
  (bind _output_get (Variables|Default|SetHealth (- (Variables|Default|GetHealth) Damage)))
  (bind _asascension (Utilities|Casting|CastToAscension (Game|GetGameInstance)))
  (Variables|/Game/Ascension.Ascension_C|SetPlayerHealth _asascension _output_get)
  (Character|LaunchCharacter (* (* HitNormal Damage) -5e+01) true true)
  (Effects|SpawnEmitterAttached "/Game/StarterContent/Particles/P_Explosion.P_Explosion" (Variables|Default|GetSprite) "None")
  (Sprite|SetSpriteColor "(R=0.905000,G=0.000000,B=0.000000,A=1.000000)")
  (Utilities|FlowControl|Delay 0.5)
  (Sprite|SetSpriteColor "(R=1.000000,G=1.000000,B=1.000000,A=1.000000)")
  (bind _output_get_2 (Variables|Default|SetIsDead (<= (Variables|Default|GetHealth) 0.0)))
  (CallFunction|UpdateAnimation)
  (if _output_get_2
    (Utilities|FlowControl|DoOnce false
      (:Completed
        (Pawn|Components|CharacterMovement|DisableMovement)
        ;;[1 1 1] Show Restart Game Widget
        (bind _returnvalue (UserInterface|CreateWidget "/Game/Blueprints/RestarGame.RestarGame_C"))
        (UserInterface|Viewport|AddtoViewport _returnvalue 0)
        (Variables|/Script/Engine.PlayerController|SetbShowMouseCursor (Game|GetPlayerController 0) false)))))

(event EventOnLanded
  (params (Hit :type Hit%20Result%20Structure%20%28by%20ref%29))
  ;[1 1 1] Jumping
  (Variables|Default|SetJumpCount 0))

(event Input|ActionEvents|InputActionJump
  ;[1 1 1] Jumping
  (:Pressed
    (if (<= (Variables|Default|GetJumpCount) 1)
      (Variables|Default|SetJumpCount (+ 1 (Variables|Default|GetJumpCount)))
      (Character|Jump)))
  (:Released
    (Character|StopJumping)))

(event Input|ActionEvents|InputActionAttack
  (bind _attackflipbook (Variables|Animations|GetAttackFlipbook))
  (bind _returnvalue (Class|PaperFlipbook|GetTotalDuration _attackflipbook))
  ;[1 1 1] Handle attacking
  (:Pressed
    (Variables|Default|SetIs%20Attacking true)
    (CallFunction|UpdateAnimation)
    (Utilities|FlowControl|Delay (/ _returnvalue 3.0))
    (for _array_element (Collision|GetOverlappingActors (Variables|Default|GetswordHitBox) "/Script/Paper2D.PaperCharacter" :!class /Script/Engine.PrimitiveComponent)
      (CallFunction|SwordHit _array_element))
    (for _array_element_2 (Collision|GetOverlappingActors (Variables|Default|GetswordHitBox2) "/Script/Paper2D.PaperCharacter" :!class /Script/Engine.PrimitiveComponent)
      (CallFunction|SwordHit _array_element_2))
    (Utilities|FlowControl|Delay (/ _returnvalue 1.5))
    (Variables|Default|SetIs%20Attacking false)
    (CallFunction|UpdateAnimation)))

(event Input|AxisEvents|InputAxisMoveRight
  (params (AxisValue :type Float%20%28single-precision%29))
  ;[1 1 1] Movement
  (Pawn|Input|AddMovementInput "1.000000, 0, 0" AxisValue false)
  (CallFunction|UpdateAnimation)
  (Math|Float|CompareFloat AxisValue 0.0
    (:>
      (Pawn|SetControlRotation (Pawn|GetController) (Class|KismetMathLibrary|MakeRot 0.0 1.8e+02 0.0)))
    (:<
      (Pawn|SetControlRotation (Pawn|GetController) (Class|KismetMathLibrary|MakeRot 0.0 0.0 0.0)))))

(event Input|KeyboardEvents|R
  ;[1 1 1] Reset Level
  (:Pressed
    (if (Variables|Default|GetIsDead)
      (bind _asascension (Utilities|Casting|CastToAscension (Game|GetGameInstance)))
      (Widget|RemovefromParent (stale EventPointDamage _returnvalue))
      (Game|OpenLevel(byName) (Variables|/Game/Ascension.Ascension_C|GetCurrentLevel _asascension)))))

(event Input|KeyboardEvents|A
  ;[1 1 1] Running, jumping, and attack sounds
  (:Pressed
    (Class|GameplayStatics|PlaySoundAttached "/Game/Sounds/sword_slash_Cue.sword_slash_Cue" (Variables|Default|GetSprite))))

(event Input|KeyboardEvents|SpaceBar
  ;[1 1 1] Running, jumping, and attack sounds
  (:Pressed
    (Class|GameplayStatics|PlaySoundAttached "/Game/Sounds/JumpSound.JumpSound" (Variables|Default|GetSprite))))

(event Input|KeyboardEvents|Left
  ;[1 1 1] Running, jumping, and attack sounds
  (:Pressed
    (bind _returnvalue (Class|GameplayStatics|PlaySoundAttached "/Game/Sounds/running_Cue.running_Cue" (Variables|Default|GetSprite))))
  (:Released
    (Audio|Components|Audio|Stop _returnvalue)))

(event Input|KeyboardEvents|Right
  ;[1 1 1] Running, jumping, and attack sounds
  (:Pressed
    (bind _returnvalue (Class|GameplayStatics|PlaySoundAttached "/Game/Sounds/running_Cue.running_Cue" (Variables|Default|GetSprite))))
  (:Released
    (Audio|Components|Audio|Stop _returnvalue)))

(fn ConstructionScript
  ;[1 1 1] Lower Jump Velocity
  (Variables|/Script/Engine.CharacterMovementComponent|SetJumpZVelocity (Variables|Character|GetCharacterMovement) 7e+02)
  ;[1 1 1] Set Player Health
  (bind _asascension (Utilities|Casting|CastToAscension (Game|GetGameInstance)))
  (Variables|Default|SetHealth (Variables|/Game/Ascension.Ascension_C|GetPlayerHealth _asascension)))

(fn AnimationStateMachine
  (params (IsFalling :type Boolean :default false) (IsMoving :type Boolean :default false) (IsDead :type Boolean :default false) (IsAttacking :type Boolean :default false))
  ;[1 1 1] Collect data
  (LocalVariables|SetIsFallingLocal IsFalling)
  (LocalVariables|SetIsMovingLocal IsMoving)
  (LocalVariables|SetIsDeadLocal IsDead)
  (LocalVariables|SetIsAttackingLocal IsAttacking)
  ;[1 1 1] Test data
  (|TestforDeath
    (:then
      ;[1 1 1] Set Animation State
      (LocalVariables|SetAnimationState "NewEnumerator3"))
    (:else
      (|TestforAttacking
        (:then
          (LocalVariables|SetAnimationState "NewEnumerator4"))
        (:else
          (|TestForJumping
            (:then
              (LocalVariables|SetAnimationState "NewEnumerator2"))
            (:else
              (|TestForRunningorIdle
                (:then
                  (LocalVariables|SetAnimationState "NewEnumerator1"))
                (:else
                  (LocalVariables|SetAnimationState "NewEnumerator0")))))))))
  (return (Utilities|Select :Index (LocalVariables|GetAnimationState) :NewEnumerator0 (Variables|Animations|GetIdleFlipbook) :NewEnumerator1 (Variables|Animations|GetRunFlipbook) :NewEnumerator2 (Variables|Animations|GetJumpFlipbook) :NewEnumerator3 (Variables|Animations|GetDeathFlipbook) :NewEnumerator4 (Variables|Animations|GetAttackFlipbook))))