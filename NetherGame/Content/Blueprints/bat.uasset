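; Flying Paper2D bat enemy that chases the player and deals contact damage.
; Tick steers toward the player when near; otherwise it wanders randomly on the XZ plane, pulled back toward its spawn point when too far.
; Damage updates the health bar widget, applies knockback, spawns an explosion and flashes the sprite red.
; At zero HP it drops and is destroyed after a delay, with flipbooks following idle, move and dead states.
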(event `self.ReceiveAnyDamage`
  (params (Damage :type "Float (single-precision)") (DamageType :type "DamageType Object Reference") (InstigatedBy :type "Controller Object Reference") (DamageCauser :type "Actor Object Reference"))
  (bind _sprite (`self.Sprite`))
  ;[1 1 1] Take Damage
  (bind _output_get (set `self.HP` (- (`self.HP`) Damage)))
  (`CharacterMovementComponent.AddImpulse` (* (* (`KismetMathLibrary.GetDirectionVector` (`self.K2_GetActorLocation` DamageCauser) (`self.K2_GetActorLocation` self)) Damage) 2000.0))
  (`self.updateHPBar`)
  (`GameplayStatics.SpawnEmitterAttached` "/Game/StarterContent/Particles/P_Explosion.P_Explosion" _sprite)
  (`PaperFlipbookComponent.SetSpriteColor` _sprite (struct :`R` 0.905 :`A` 1.0))
  (`KismetSystemLibrary.Delay` 0.5)
  (`PaperFlipbookComponent.SetSpriteColor` _sprite (struct :`R` 1.0 :`G` 1.0 :`B` 1.0 :`A` 1.0))
  (set `self.isDead` (<= _output_get 0.0))
  (`self.Update Animation`)
  (`MovementComponent.StopMovementImmediately`))

(event `self.ReceiveHit`
  (params (MyComp :type "PrimitiveComponent Object Reference") (Other :type "Actor Object Reference") (OtherComp :type "PrimitiveComponent Object Reference") (bSelfMoved :type Boolean) (HitLocation :type "Object.Vector Structure") (HitNormal :type "Object.Vector Structure") (NormalImpulse :type "Object.Vector Structure") (Hit :type "EngineTypes.HitResult Structure (by ref)"))
  ;[1 1 1] Apply damage to things it touches
  (cast `/Game/Blueprints/MyCharacter` Other)
  (`GameplayStatics.ApplyPointDamage` Other 20.0 HitNormal Hit null self)
  (`self.LaunchCharacter` (* HitNormal 300.0)))

(event `self.ReceiveTick`
  (params (DeltaSeconds :type "Float (single-precision)"))
  (bind _returnvalue (`GameplayStatics.GetPlayerCharacter` 0))
  (bind _returnvalue_2 (`self.K2_GetActorLocation`))
  (bind _startingloc (`self.startingLoc`))
  (`CharacterMovementComponent.SetMovementMode` "MOVE_Flying")
  (if (`self.isDead`)
    ;[1 1 1] Falls and dies
    (`self.fallanddie`)
    (`KismetSystemLibrary.Delay` 1.0)
    (`self.K2_DestroyActor`)
    (else
      ;[1 1 1] Moves Towards Player
      (if (<= (`self.GetDistanceTo` _returnvalue) 750.0)
        (`PawnMovementComponent.AddInputVector` (`self.CharacterMovement`) (* (`KismetMathLibrary.GetDirectionVector` (`self.K2_GetActorLocation`) (`self.K2_GetActorLocation` _returnvalue)) 0.5) false)
        (set `self.isMovingRandomly` false)
        (`self.Update Animation`)
        (else
          (if (>= (`KismetMathLibrary.VSize` (- _startingloc _returnvalue_2)) 500.0)
            (`PawnMovementComponent.AddInputVector` (`KismetMathLibrary.GetDirectionVector` _returnvalue_2 _startingloc))
            (else
              (`PawnMovementComponent.AddInputVector` (`KismetMathLibrary.MakeVector` (.x (`KismetMathLibrary.RandomUnitVector`)) 0.0 (.z (`KismetMathLibrary.RandomUnitVector`))))
              (set `self.isMovingRandomly` true)))
          (`self.Update Animation`))))))

(event `self.ReceiveBeginPlay`)

(event `self.ReceiveActorBeginOverlap`
  (params (OtherActor :type "Actor Object Reference")))

(event `Update Animation`
  (bind _ismovingrandomly (`self.isMovingRandomly`))
  ;[1 1 1] Update minion animation
  (if (`self.isDead`)
    (`PaperFlipbookComponent.SetFlipbook` "/Game/FlipBooks/bat_dead_Flipbook.bat_dead_Flipbook")
    (else
      (if _ismovingrandomly
        (`PaperFlipbookComponent.SetFlipbook` (`self.Sprite`) "/Game/FlipBooks/bat_idle_Flipbook.bat_idle_Flipbook")
        (else
          (`PaperFlipbookComponent.SetFlipbook` (`self.Sprite`) "/Game/FlipBooks/bat_move_Flipbook.bat_move_Flipbook")))
      (`SceneComponent.K2_SetWorldRotation` (`self.Sprite`) (`KismetMathLibrary.MakeRot` 180.0 (`KismetMathLibrary.SelectFloat` 180.0 0.0 (and (not _ismovingrandomly) (>= (.x (`PawnMovementComponent.GetLastInputVector` (`self.CharacterMovement`))) 0.0))) 180.0) false))))

(fn `fallanddie`
  (`self.AddMovementInput` (0.0 0.0 -1.0) 50.0 true))

(fn `updateHPBar`
  (bind _asenemy_health (cast `/Game/Blueprints/enemyHealth` (`WidgetComponent.GetUserWidgetObject`))
    (:`then`
      (`ProgressBar.SetPercent` (`/Game/Blueprints/enemyHealth.hpBar` _asenemy_health) (/ (`self.HP`) (`self.MaxHp`))))
    (:`CastFailed`
      _))
  (return))

(fn `UserConstructionScript`
  (set `self.HP` 100.0)
  (set `self.MaxHp` 100.0)
  (`CharacterMovementComponent.SetMovementMode` (`self.CharacterMovement`) "MOVE_Flying" 0)
  (set `self.startingLoc` (`self.K2_GetActorLocation`)))