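; Enemy mummy character for a side-view sprite game that patrols back and forth along X and hurts the player on contact.
; Tick drives movement through a DoN counter that reverses direction after the patrol distance, flipping the sprite to match.
; Hits deal point damage to the player and launch the mummy along the hit normal.
; Taking damage applies knockback, updates a widget health bar, flashes red, and at zero HP destroys it and awards score.
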(event `self.ReceiveAnyDamage`
  (params (Damage :type "Float (single-precision)") (DamageType :type "DamageType Object Reference") (InstigatedBy :type "Controller Object Reference") (DamageCauser :type "Actor Object Reference"))
  (bind _sprite (`self.Sprite`))
  ;[1 1 1] Take Damage
  (`GameplayStatics.PlaySoundAttached` "/Game/Sounds/hit_enemy_Cue.hit_enemy_Cue" (`self.Sprite`))
  (bind _output_get (set `self.HP` (- (`self.HP`) Damage)))
  (`CharacterMovementComponent.AddImpulse` (* (* (`KismetMathLibrary.GetDirectionVector` (`self.K2_GetActorLocation` DamageCauser) (`self.K2_GetActorLocation` self)) Damage) 10000.0))
  (`self.updateHPBar`)
  (`GameplayStatics.SpawnEmitterAttached` "/Game/StarterContent/Particles/P_Explosion.P_Explosion" _sprite)
  (`PaperFlipbookComponent.SetSpriteColor` _sprite (struct :`R` 0.905 :`A` 1.0))
  (`KismetSystemLibrary.Delay` 0.5)
  (`PaperFlipbookComponent.SetSpriteColor` _sprite (struct :`R` 1.0 :`G` 1.0 :`B` 1.0 :`A` 1.0))
  (if (<= _output_get 0.0)
    (`GameplayStatics.SpawnEmitterAtLocation` "/Game/StarterContent/Particles/P_Explosion.P_Explosion" (`self.K2_GetActorLocation`))
    (`self.K2_DestroyActor` self)
    ;[1 1 1] Add score
    (bind _asmy_character (cast `/Game/Blueprints/MyCharacter` (`GameplayStatics.GetPlayerCharacter` 0)))
    (set `/Game/Blueprints/MyCharacter.score` (+ (`/Game/Blueprints/MyCharacter.score` _asmy_character) 10) _asmy_character)))

(event `self.ReceiveHit`
  (params (MyComp :type "PrimitiveComponent Object Reference") (Other :type "Actor Object Reference") (OtherComp :type "PrimitiveComponent Object Reference") (bSelfMoved :type Boolean) (HitLocation :type "Object.Vector Structure") (HitNormal :type "Object.Vector Structure") (NormalImpulse :type "Object.Vector Structure") (Hit :type "EngineTypes.HitResult Structure (by ref)"))
  ;[1 1 1] Apply damage to things it touches
  (cast `/Game/Blueprints/MyCharacter` Other)
  (`GameplayStatics.ApplyPointDamage` Other 20.0 HitNormal Hit null self)
  (`self.LaunchCharacter` (* HitNormal 300.0)))

(event `self.ReceiveTick`
  (params (DeltaSeconds :type "Float (single-precision)"))
  (bind _patroldistance (`self.PatrolDistance`))
  ;[1 1 1] Patrol
  (bind _counter (`/Engine/EditorBlueprintResources/StandardMacros.Do N` _patroldistance :!label _label)
    (:`Exit`
      (if (== _counter _patroldistance)
        (set `self.mummyDir` (* (`self.mummyDir`) -1.0))
        (goto _label :!via `Reset`)
        (else
          (`PawnMovementComponent.AddInputVector` (`self.CharacterMovement`) (* (* (`KismetMathLibrary.MakeVector` 1.0) (`self.mummyDir`)) 0.75) false)
          (`self.Update Animation`))))))

(event `self.ReceiveActorBeginOverlap`
  (params (OtherActor :type "Actor Object Reference")))

(event `Update Animation`
  ;[1 1 1] Update mummy
  ;  animation
  (`SceneComponent.K2_SetWorldRotation` (`self.Sprite`) (`KismetMathLibrary.MakeRot` 180.0 (`KismetMathLibrary.SelectFloat` 0.0 180.0 (>= (.x (`PawnMovementComponent.GetLastInputVector` (`self.CharacterMovement`))) 0.0)) 180.0) false))

(fn `updateHPBar`
  (bind _asenemy_health (cast `/Game/Blueprints/enemyHealth` (`WidgetComponent.GetUserWidgetObject`))
    (:`then`
      (`ProgressBar.SetPercent` (`/Game/Blueprints/enemyHealth.hpBar` _asenemy_health) (/ (`self.HP`) (`self.MaxHp`))))
    (:`CastFailed`
      _))
  (return))

(fn `UserConstructionScript`
  (set `self.HP` 100.0)
  (set `self.MaxHp` 100.0))