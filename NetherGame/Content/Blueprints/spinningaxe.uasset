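; Spinning axe projectile actor that damages the player character type, MyCharacter, on overlap.
; Each Tick teleports it a fixed step opposite its forward vector, so its speed depends on frame rate; the graph applies no rotation.
; Overlapping a MyCharacter applies fixed point damage along the axe's forward vector, then destroys the axe, while other actors are ignored.
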(event `self.ReceiveBeginPlay`)

(event `self.ReceiveActorBeginOverlap`
  (params (OtherActor :type "Actor Object Reference"))
  (bind _asmy_character (cast `/Game/Blueprints/MyCharacter` OtherActor))
  (`GameplayStatics.ApplyPointDamage` _asmy_character 50.0 (`KismetMathLibrary.Conv_RotatorToVector` (`self.K2_GetActorRotation`)) (`self.dummyHit`) null self)
  (`self.K2_DestroyActor`))

(event `self.ReceiveTick`
  (params (DeltaSeconds :type "Float (single-precision)"))
  (bind _returnvalue (`self.K2_GetActorRotation`))
  (`self.K2_TeleportTo` (- (`self.K2_GetActorLocation`) (* (`KismetMathLibrary.Conv_RotatorToVector` _returnvalue) 10.0)) _returnvalue))

(fn `UserConstructionScript`)